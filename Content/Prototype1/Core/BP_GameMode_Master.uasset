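; BP_GameMode_Master is the prototype's core game mode, which caps the frame rate on BeginPlay and offers battle debug helpers.
; SetFPSLimit stores the limit and applies it through GameUserSettings.
; A DebugSettings variable, exposed by a getter, gates on-screen prints of enemy count and character HP and initiative.
; GetCurrentHero and SetCurrentHero are empty stubs, with the setter always returning false.
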(event `self.ReceiveBeginPlay`
  (`self.SetFPSLimit` 60.0))

(fn `Debug_ShowBasicStats`
  (params (Name :type "Text (by ref)") (HP :type Integer) (HP_Max :type Integer) (Init :type "Float (double-precision)"))
  (if (`.Battle_CharacterStats_12_1EDFF5C44C8FE5CE0FCE2C9F6037E3B0` (break `/Game/Prototype1/Core/Structures/Settings/S_DebugSettings` (`self.DebugSettings`)))
    (`KismetSystemLibrary.PrintString` (`KismetStringLibrary.Concat_StrStr` (`KismetTextLibrary.Conv_TextToString` Name) " :     HP : " (`KismetStringLibrary.Conv_IntToString` HP) "     " "    HP Max : " (`KismetStringLibrary.Conv_IntToString` HP_Max) "    Init : " (`KismetStringLibrary.Conv_DoubleToString` Init)) true true (struct :`G` 0.66 :`B` 1.0 :`A` 1.0) 20.0)
    (return)))

(fn `GetCurrentHero`
  (returns (Return :type "/Game/Prototype1/Core/Characters/BP_CharacterBase_Master Object Reference"))
  (return null))

(fn `GetDebugSettings`
  (returns (DebugStructure :type "/Game/Prototype1/Core/Structures/Settings/S_DebugSettings Structure"))
  (return (`self.DebugSettings`)))

(fn `SetCurrentHero`
  (params (HeroUnit :type "/Game/Prototype1/Core/Characters/BP_CharacterBase_Master Object Reference"))
  (returns (UnusedReturn :type Boolean))
  (return false))

(fn `SetFPSLimit`
  (params (RateLimit :type "Float (single-precision)"))
  (bind _output_get (set `self.FPSLimit` RateLimit))
  (bind _returnvalue (`GameUserSettings.GetGameUserSettings`))
  (`GameUserSettings.SetFrameRateLimit` _returnvalue _output_get)
  (`GameUserSettings.ApplyNonResolutionSettings` _returnvalue)
  (return))

(fn `ShowDebug`
  (`|ExecutionSequence`
    (:`then_0`
      (if (`.Battle_EnemyNumber_15_5FD2CE164E7358D6FFE08BB2C1A8DA92` (break `/Game/Prototype1/Core/Structures/Settings/S_DebugSettings` (`self.DebugSettings`)))
        (`KismetSystemLibrary.PrintString` (`KismetStringLibrary.Concat_StrStr` "Enemy Number = " (`KismetStringLibrary.Conv_IntToString` (+ (`self.Enemy Per Battle`) 1))) true true (struct :`G` 0.66 :`B` 1.0 :`A` 1.0) 20.0)))
    (:`then_2`
      (return))))

(fn `UserConstructionScript`)