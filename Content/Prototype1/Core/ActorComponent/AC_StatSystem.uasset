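; Actor component that holds and edits RPG attributes and stats for a BP_CharacterBase_Master owner.
; BeginPlay loads CharacterStats from the character or enemy DataTable by name, then refreshes each attribute to compute totals.
; Modify functions route through clamped setters, with non-Level attribute totals combining dice roll, scale, base value and bonuses, including job bonuses from a table.
; Random-gain level-up is marked old with its timer unwired, and ScalingStats is unfinished.
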(event `self.ReceiveBeginPlay`
  (bind _asbp_character_base_master (cast `/Game/Prototype1/Core/Characters/BP_CharacterBase_Master` (`self.GetOwner`)))
  (set `self.UnitCharacter` _asbp_character_base_master)
  (`self.Set_CharacterStats`)
  ; Temporary
  (for _array_element (`.Attribute_42_8D9DAF1543FFD03492ED8C95A5DE525D` (break `/Game/Prototype1/Core/Structures/S_Character_Stats` (`self.Character_Stats`)))
    (`self.ModifyAttribute` "NewEnumerator0" "NewEnumerator1" (`.Name_6_9990C3F841326096ECE18BA5E76876A9` (break `/Game/Prototype1/Core/Structures/Stats_Struc/S_SingleAttibutes` _array_element)) 0.0)))

(event `UpLevel`
  ; OLD
  (`self.SetAttribute` "NewEnumerator1" "NewEnumerator0" (+ (`self.GetAttributeValue` "NewEnumerator1") 1.0))
  (`self.OLD_LevelUpAttributeCurrent`))

(fn `GetAttributeBonus`
  (params (Attribute :type "/Game/Prototype1/Core/Enum/Stat_Enum/E_Stat_AttributeList Enum" :default "NewEnumerator0"))
  (returns (ReturnValue :type "Float (double-precision)"))
  (return (+ (`self.GetAttributeJobBonus` Attribute) 0.0)))

(fn `GetAttributeDice`
  (params (Attribute :type "/Game/Prototype1/Core/Enum/Stat_Enum/E_Stat_AttributeList Enum" :default "NewEnumerator0"))
  (returns (ReturnValue :type "Float (double-precision)"))
  (bind _returnvalue (`/Game/Prototype1/Core/FL_FunctionLibrary.Dice_Custom` (`.Dice_42_27E097BC4278D66F08D94C8DD3BA68D9` (break `/Game/Prototype1/Core/Structures/Stats_Struc/S_SingleAttibutes` (`self.GetAttributeRef` Attribute)))))
  (return (`KismetMathLibrary.Conv_IntToDouble` _returnvalue)))

(fn `GetAttributeJobBonus`
  (params (Attribute :type "/Game/Prototype1/Core/Enum/Stat_Enum/E_Stat_AttributeList Enum" :default "NewEnumerator0"))
  (returns (ReturnValue :type "Float (double-precision)"))
  (bind _returnvalue (`|GetDataTableRow` "/Game/Prototype1/Core/Structures/Stats_Struc/DT_Stat_Jobs.DT_Stat_Jobs" (`KismetStringLibrary.Conv_StringToName` (`|GetEnumeratorNameAsString` (`.Job_40_FBD99DE842F4748849277D9B871DA84D` (break `/Game/Prototype1/Core/Structures/S_Character_Stats` (`self.Character_Stats`))))))
    (:`then`
      (return (`BlueprintMapLibrary.Map_Find` (`.JobAttributBonus_34_AF49944142C11EF48CEB99BB2E8DCF3B` (break `/Game/Prototype1/Core/Structures/Stats_Struc/S_SingleJob` _returnvalue)) (`.JobBonus_67_2BA4FB274D29CA9166F8CAB87436AAB4` (break `/Game/Prototype1/Core/Structures/Stats_Struc/S_SingleAttibutes` (`self.GetAttributeRef` Attribute))))))))

(fn `GetAttributeRef`
  (params (Attribute :type "/Game/Prototype1/Core/Enum/Stat_Enum/E_Stat_AttributeList Enum" :default "NewEnumerator0"))
  (returns (ResultAttribute :type "/Game/Prototype1/Core/Structures/Stats_Struc/S_SingleAttibutes Structure") (ResultIndex :type Integer))
  (locals (L_AttributeValue :type "/Game/Prototype1/Core/Structures/Stats_Struc/S_SingleAttibutes Structure") (L_AttributeIndex :type Integer))
  (for (_array_element _array_index) (`.Attribute_42_8D9DAF1543FFD03492ED8C95A5DE525D` (break `/Game/Prototype1/Core/Structures/S_Character_Stats` (`self.Character_Stats`)))
    (set `local.L_AttributeValue` _array_element)
    (set `local.L_AttributeIndex` _array_index)
    (if (`|EnumEquality` (`local.Attribute`) (`.Name_6_9990C3F841326096ECE18BA5E76876A9` (break `/Game/Prototype1/Core/Structures/Stats_Struc/S_SingleAttibutes` _array_element)))
      (return (`local.L_AttributeValue`) (`local.L_AttributeIndex`)))))

(fn `GetAttributeValue`
  (params (Type :type "/Game/Prototype1/Core/Enum/Stat_Enum/E_Attribute_Type Enum" :default "NewEnumerator0") (Attribute :type "/Game/Prototype1/Core/Enum/Stat_Enum/E_Stat_AttributeList Enum" :default "NewEnumerator0"))
  (returns (ReturnValue :type "Float (double-precision)"))
  (bind ((`Default_22_044B8F4C46F014FCB6F990B53504DDC0` _default) (`Bonus_68_5ED13924472C87117E5B838E8D6A28F4` _bonus) (`Total_65_63AA6356417A02B4DB41FCA0E9A83F11` _total) (`Final_21_F97B0B0440B7C2925AECE09DDEEA5C7F` _final) (`Scale_27_0EDB51594481C41F3669B7ACE5C9E27A` _scale)) (break `/Game/Prototype1/Core/Structures/Stats_Struc/S_SingleAttibutes` (`self.GetAttributeRef` Attribute)))
  (return (select `/Game/Prototype1/Core/Enum/Stat_Enum/E_Attribute_Type` (`local.Type`) :`NewEnumerator0` -1.0 :`NewEnumerator1` _default :`NewEnumerator7` _bonus :`NewEnumerator8` _total :`NewEnumerator14` _final :`NewEnumerator13` _scale)))

(fn `GetGainMax`
  (params (Attribute :type "/Game/Prototype1/Core/Enum/Stat_Enum/E_Stat_AttributeList Enum" :default "NewEnumerator0"))
  (returns (ReturnValue :type "Float (double-precision)"))
  (return (`KismetMathLibrary.FMax` (+ (/ (`self.GetGainRemaining` Attribute) (`self.GetGainRemaining` "NewEnumerator0")) 1.0) (`self.GetGainMin` (`local.Attribute`)))))

(fn `GetGainMin`
  (params (Attribute :type "/Game/Prototype1/Core/Enum/Stat_Enum/E_Stat_AttributeList Enum" :default "NewEnumerator0"))
  (returns (ReturnValue :type "Float (double-precision)"))
  (return 0.0))

(fn `GetGainRemaining`
  (params (Attribute :type "/Game/Prototype1/Core/Enum/Stat_Enum/E_Stat_AttributeList Enum" :default "NewEnumerator0"))
  (returns (ReturnValue :type "Float (double-precision)"))
  (return (- (`self.GetAttributeValue` "NewEnumerator14" Attribute) (`self.GetAttributeValue` "NewEnumerator8" Attribute))))

(fn `GetGainResult`
  (params (Attribute :type "/Game/Prototype1/Core/Enum/Stat_Enum/E_Stat_AttributeList Enum" :default "NewEnumerator0"))
  (returns (ReturnValue :type "Float (double-precision)"))
  (return (`KismetMathLibrary.RandomFloatInRange` (`self.GetGainMin` Attribute) (`self.GetGainMax` Attribute))))

(fn `GetStatDefault`
  (params (Stat :type "/Game/Prototype1/Core/Enum/Stat_Enum/E_Stat_List Enum" :default "NewEnumerator23"))
  (returns (Result :type "Float (double-precision)"))
  (return (/ (* (`self.GetStatValue` "NewEnumerator13" Stat) (`self.GetStatValue` "NewEnumerator14" Stat)) 2.0)))

(fn `GetStatDice`
  (params (Stat :type "/Game/Prototype1/Core/Enum/Stat_Enum/E_Stat_List Enum" :default "NewEnumerator23"))
  (returns (ReturnValue :type "Float (double-precision)"))
  (bind _returnvalue (`/Game/Prototype1/Core/FL_FunctionLibrary.Dice_Custom` (`.Dice_47_D32C77B442E725F5C636D088457D3E8B` (break `/Game/Prototype1/Core/Structures/Stats_Struc/S_SingleStat` (`self.GetStatRef` Stat)))))
  (return (`KismetMathLibrary.Conv_IntToDouble` _returnvalue)))

(fn `GetStatRef`
  (params (Stat :type "/Game/Prototype1/Core/Enum/Stat_Enum/E_Stat_List Enum" :default "NewEnumerator23"))
  (returns (ResultStat :type "/Game/Prototype1/Core/Structures/Stats_Struc/S_SingleStat Structure") (ResultIndex :type Integer))
  (locals (L_StatIndex :type Integer) (L_StatValue :type "/Game/Prototype1/Core/Structures/Stats_Struc/S_SingleStat Structure"))
  (for (_array_element _array_index) (`.Stat_46_561705244D810CB8FD450891CBFE6803` (break `/Game/Prototype1/Core/Structures/S_Character_Stats` (`self.Character_Stats`)))
    (set `local.L_StatValue` _array_element)
    (set `local.L_StatIndex` _array_index)
    (if (`|EnumEquality` (`local.Stat`) (`.Name_6_9990C3F841326096ECE18BA5E76876A9` (break `/Game/Prototype1/Core/Structures/Stats_Struc/S_SingleStat` _array_element)))
      (return (`local.L_StatValue`) (`local.L_StatIndex`)))))

(fn `GetStatValue`
  (params (Type :type "/Game/Prototype1/Core/Enum/Stat_Enum/E_Stat_Type Enum" :default "NewEnumerator0") (Stat :type "/Game/Prototype1/Core/Enum/Stat_Enum/E_Stat_List Enum" :default "NewEnumerator23"))
  (returns (ReturnValue :type "Float (double-precision)"))
  (bind ((`Current_22_5301AE1F4A59B76037ACD09D2FB07A42` _current) (`Extra_37_8B0A353944345F1210B69E8330BC27D8` _extra) (`Total_24_5991D9BE423260CF8083B08FCBBE45C6` _total) (`Final_26_B6CF407644F1FAECB10B66BCF3267972` _final) (`Default_28_181A231549871FDB2E3D5D8EBABF76C8` _default) (`Power_16_5A23B7CF4392019815203DAB03FCF5CA` _power) (`Scale_36_2847FE694979D4E932A28DAA309717F1` _scale) (`Base_46_6B4FBEDB4DAC43D99B2578B868764F17` _base) (`BaseMult_45_6BA2BAF5444749EA58662E9D7655D759` _basemult)) (break `/Game/Prototype1/Core/Structures/Stats_Struc/S_SingleStat` (`self.GetStatRef` Stat)))
  (return (select `/Game/Prototype1/Core/Enum/Stat_Enum/E_Stat_Type` (`local.Type`) :`NewEnumerator0` -1.0 :`NewEnumerator1` _current :`NewEnumerator5` _extra :`NewEnumerator2` _total :`NewEnumerator7` _final :`NewEnumerator8` _default :`NewEnumerator12` _power :`NewEnumerator10` _scale :`NewEnumerator13` _base :`NewEnumerator14` _basemult)))

(fn `GetXpBase`
  (returns (ReturnValue :type "Float (double-precision)"))
  (return (/ (`self.GetStatValue` "NewEnumerator7" "NewEnumerator0") (`self.GetStatValue` "NewEnumerator10" "NewEnumerator0"))))

(fn `GetXpNextLevel`
  (returns (ReturnNextLevelXp :type "Float (double-precision)"))
  (return (`KismetMathLibrary.Conv_IntToDouble` (`KismetMathLibrary.FFloor` (* (`self.GetXpBase`) (`KismetMathLibrary.Square` (`self.GetAttributeValue` "NewEnumerator1")))))))

(fn `ModifyAttribute`
  (params (Operation :type "/Game/Prototype1/Core/Enum/Stat_Enum/E_Stat_Operations Enum" :default "NewEnumerator0") (Type :type "/Game/Prototype1/Core/Enum/Stat_Enum/E_Attribute_Type Enum" :default "NewEnumerator0") (Attribute :type "/Game/Prototype1/Core/Enum/Stat_Enum/E_Stat_AttributeList Enum" :default "NewEnumerator0") (Value :type "Float (double-precision)"))
  (bind _value (`local.Value`))
  (bind _returnvalue (`self.GetAttributeValue` (`local.Type`) (`local.Attribute`)))
  (switch `/Game/Prototype1/Core/Enum/Stat_Enum/E_Attribute_Type` Type
    (:`NewEnumerator0`
      (`KismetSystemLibrary.PrintString` "Warning: Modify Attribute - \nerror Attribute is set to \"None\"")
      (return))
    (:`NewEnumerator1`
      _)
    (:`NewEnumerator7`
      _)
    (:`NewEnumerator8`
      (`self.OperateTotalAttribute` (`local.Operation`) (`local.Attribute`) (`local.Value`))
      (return)))
  (`self.SetAttribute` (`local.Type`) (`local.Attribute`) (select `/Game/Prototype1/Core/Enum/Stat_Enum/E_Stat_Operations` (`local.Operation`) :`NewEnumerator0` (+ _returnvalue _value) :`NewEnumerator1` (- _returnvalue _value) :`NewEnumerator2` _value))
  (return))

(fn `ModifyStat`
  (params (Operation :type "/Game/Prototype1/Core/Enum/Stat_Enum/E_Stat_Operations Enum" :default "NewEnumerator0") (Type :type "/Game/Prototype1/Core/Enum/Stat_Enum/E_Stat_Type Enum" :default "NewEnumerator0") (Stat :type "/Game/Prototype1/Core/Enum/Stat_Enum/E_Stat_List Enum" :default "NewEnumerator23") (Value :type "Float (double-precision)"))
  (bind _value (`local.Value`))
  (bind _returnvalue (`self.GetStatValue` (`local.Type`) (`local.Stat`)))
  (switch `/Game/Prototype1/Core/Enum/Stat_Enum/E_Stat_Type` Type
    (:`NewEnumerator0`
      (`KismetSystemLibrary.PrintString` "Warning: Modify Attribute - \nerror Attribute is set to \"None\"")
      (return))
    (:`NewEnumerator1`
      _)
    (:`NewEnumerator5`
      _)
    (:`NewEnumerator2`
      (`self.OperateTotalStat` (`local.Operation`) (`local.Stat`) (`local.Value`))
      (return))
    (:`NewEnumerator7`
      _)
    (:`NewEnumerator8`
      _)
    (:`NewEnumerator12`
      _)
    (:`NewEnumerator10`
      _))
  (`self.SetStat` (`local.Type`) (`local.Stat`) (select `/Game/Prototype1/Core/Enum/Stat_Enum/E_Stat_Operations` (`local.Operation`) :`NewEnumerator0` (+ _returnvalue _value) :`NewEnumerator1` (- _returnvalue _value) :`NewEnumerator2` _value))
  (return))

(fn `OLD_GetLevelRemaining`
  (returns (ReturnValue :type "Float (double-precision)"))
  (return (- (`self.GetAttributeValue` "NewEnumerator14") (`self.GetAttributeValue` "NewEnumerator8"))))

(fn `OLD_LevelUpAttributeCurrent`
  (locals (L_AttributeCurrent :type "/Game/Prototype1/Core/Enum/Stat_Enum/E_Stat_AttributeList Enum"))
  (bind _l_attributecurrent (`local.L_AttributeCurrent`))
  (for _array_element (`.Attribute_42_8D9DAF1543FFD03492ED8C95A5DE525D` (break `/Game/Prototype1/Core/Structures/S_Character_Stats` (`self.Character_Stats`)))
    (bind _output_get (set `local.L_AttributeCurrent` (`.Name_6_9990C3F841326096ECE18BA5E76876A9` (break `/Game/Prototype1/Core/Structures/Stats_Struc/S_SingleAttibutes` _array_element))))
    (if (not (`|EnumEquality` _output_get "NewEnumerator0"))
      (`self.SetAttribute` "NewEnumerator1" (`local.L_AttributeCurrent`) (+ (`self.GetAttributeValue` "NewEnumerator1" _l_attributecurrent) (`KismetMathLibrary.Round` (`self.GetGainResult` _l_attributecurrent))))))
  (return))

(fn `OperateTotalAttribute`
  (params (Operation :type "/Game/Prototype1/Core/Enum/Stat_Enum/E_Stat_Operations Enum" :default "NewEnumerator0") (Attribute :type "/Game/Prototype1/Core/Enum/Stat_Enum/E_Stat_AttributeList Enum" :default "NewEnumerator0") (Value :type "Float (double-precision)"))
  (locals (L_StoredValue :type "Float (double-precision)" :default 0.0))
  (switch `/Game/Prototype1/Core/Enum/Stat_Enum/E_Stat_Operations` Operation
    (:`NewEnumerator0`
      (`self.ModifyAttribute` "NewEnumerator0" "NewEnumerator1" (`local.Attribute`) (`local.Value`))
      (return))
    (:`NewEnumerator1`
      (if (>= (- (`self.GetAttributeValue` "NewEnumerator7" (`local.Attribute`)) (`local.Value`)) 0.0)
        (`self.ModifyAttribute` "NewEnumerator1" "NewEnumerator7" (`local.Attribute`) (`local.Value`))
        (return)
        (else
          (bind _output_get (set `local.L_StoredValue` (`self.GetAttributeValue` "NewEnumerator7" (`local.Attribute`))))
          (`self.ModifyAttribute` "NewEnumerator1" "NewEnumerator7" (`local.Attribute`) _output_get)
          (`self.ModifyAttribute` "NewEnumerator1" "NewEnumerator1" (`local.Attribute`) (- (`local.Value`) (`local.L_StoredValue`)))
          (return))))
    (:`NewEnumerator2`
      (`KismetSystemLibrary.PrintString` "Warning: Operate Total Attribute \nUnable To Set \"Total\" Value")
      (return))))

(fn `OperateTotalStat`
  (params (Operation :type "/Game/Prototype1/Core/Enum/Stat_Enum/E_Stat_Operations Enum" :default "NewEnumerator0") (Stat :type "/Game/Prototype1/Core/Enum/Stat_Enum/E_Stat_List Enum" :default "NewEnumerator23") (Value :type "Float (double-precision)"))
  (locals (StoredValue :type "Float (double-precision)" :default 0.0))
  (switch `/Game/Prototype1/Core/Enum/Stat_Enum/E_Stat_Operations` Operation
    (:`NewEnumerator0`
      (`self.ModifyStat` "NewEnumerator0" "NewEnumerator1" (`local.Stat`) (`local.Value`))
      (return))
    (:`NewEnumerator1`
      (if (>= (- (`self.GetStatValue` "NewEnumerator5" (`local.Stat`)) (`local.Value`)) 0.0)
        (`self.ModifyStat` "NewEnumerator0" "NewEnumerator5" (`local.Stat`) (`local.Value`))
        (return)
        (else
          (bind _output_get (set `local.StoredValue` (`self.GetStatValue` "NewEnumerator5" (`local.Stat`))))
          (`self.ModifyStat` "NewEnumerator0" "NewEnumerator5" (`local.Stat`) _output_get)
          (`self.ModifyStat` "NewEnumerator0" "NewEnumerator1" (`local.Stat`) (- (`local.Value`) (`local.StoredValue`)))
          (return))))
    (:`NewEnumerator2`
      (`KismetSystemLibrary.PrintString` "Warning Operate Total Stat \nUnable to Set \"Total\" Value")
      (return))))

(fn `ScalingStats`
  (params (Type :type "/Game/Prototype1/Core/Enum/Stat_Enum/E_Stat_Type Enum" :default "NewEnumerator0") (Operation :type "/Game/Prototype1/Core/Enum/Stat_Enum/E_Stat_Operations Enum" :default "NewEnumerator0") (Value :type "Float (double-precision)"))
  (locals (L_Stat :type "/Game/Prototype1/Core/Structures/Stats_Struc/S_SingleStat Structure") (L_StatName :type "/Game/Prototype1/Core/Enum/Stat_Enum/E_Stat_List Enum"))
  (for _array_element (`.Stat_46_561705244D810CB8FD450891CBFE6803` (break `/Game/Prototype1/Core/Structures/S_Character_Stats` (`self.Character_Stats`)))
    (set `local.L_Stat` _array_element)
    (set `local.L_StatName` (`.Name_6_9990C3F841326096ECE18BA5E76876A9` (break `/Game/Prototype1/Core/Structures/Stats_Struc/S_SingleStat` _array_element)))))

(fn `Set_CharacterStats`
  (if (not (`/Game/Prototype1/Core/Characters/BP_CharacterBase_Master.bIsEnemy` (`self.UnitCharacter`)))
    (bind _returnvalue (`|GetDataTableRow` "/Game/Prototype1/Core/Structures/DT_CharatersProperties.DT_CharatersProperties" (`KismetStringLibrary.Conv_StringToName` (`|GetEnumeratorNameAsString` (`self.CharacterName`))))
      (:`then`
        (set `self.Character_Stats` _returnvalue)
        (return)))
    (else
      ; A voir si on garde ou si une seul data table global
      (bind _returnvalue_2 (`|GetDataTableRow` "/Game/Prototype1/Core/Structures/DT_EnemiesProperties.DT_EnemiesProperties" (`KismetStringLibrary.Conv_StringToName` (`|GetEnumeratorNameAsString` (`self.CharacterName`))))
        (:`then`
          (set `self.Character_Stats` _returnvalue_2)
          (return))))))

(fn `SetAttribute`
  (params (Type :type "/Game/Prototype1/Core/Enum/Stat_Enum/E_Attribute_Type Enum" :default "NewEnumerator0") (Attribute :type "/Game/Prototype1/Core/Enum/Stat_Enum/E_Stat_AttributeList Enum" :default "NewEnumerator0") (Value :type "Float (double-precision)"))
  (locals (L_Attribute :type "/Game/Prototype1/Core/Structures/Stats_Struc/S_SingleAttibutes Structure") (L_Index :type Integer :default 0) (L_Final :type "Float (double-precision)"))
  (bind (_resultattribute _resultindex) (`self.GetAttributeRef` Attribute))
  (bind _attribute (`local.Attribute`))
  (bind ((`Default_22_044B8F4C46F014FCB6F990B53504DDC0` _default)) (break `/Game/Prototype1/Core/Structures/Stats_Struc/S_SingleAttibutes` (`local.L_Attribute`)))
  (bind _returnvalue (`self.GetAttributeBonus` _attribute))
  (set `local.L_Attribute` _resultattribute)
  (set `local.L_Index` _resultindex)
  (set `local.L_Final` (`.Final_21_F97B0B0440B7C2925AECE09DDEEA5C7F` (break `/Game/Prototype1/Core/Structures/Stats_Struc/S_SingleAttibutes` (`local.L_Attribute`))))
  (switch `/Game/Prototype1/Core/Enum/Stat_Enum/E_Attribute_Type` (`local.Type`)
    (:`NewEnumerator1`
      (bind _returntotalvalue (`self.SetAttributeTotal` _attribute (`local.Value`) _returnvalue))
      (setmembers `/Game/Prototype1/Core/Structures/Stats_Struc/S_SingleAttibutes` :`StructRef` (`local.L_Attribute`) :`Default` (`KismetMathLibrary.FClamp` (`local.Value`) 0.0 (`local.L_Final`)) :`Total` (`KismetMathLibrary.FClamp` _returntotalvalue _returnvalue (`local.L_Final`))))
    (:`NewEnumerator7`
      (bind _returntotalvalue_2 (`self.SetAttributeTotal` (`local.Attribute`) _default (`local.Value`)))
      (setmembers `/Game/Prototype1/Core/Structures/Stats_Struc/S_SingleAttibutes` :`StructRef` (`local.L_Attribute`) :`Bonus` (`KismetMathLibrary.FClamp` (`local.Value`) 0.0 (`local.L_Final`)) :`Total` (`KismetMathLibrary.FClamp` _returntotalvalue_2 _default (`local.L_Final`))))
    (:`NewEnumerator8`
      (`KismetSystemLibrary.PrintString` "Warning: SetAttribute - \nError Can not use \"TOTAL\"")
      (return)))
  (`KismetArrayLibrary.Array_Set` (`.Attribute_42_8D9DAF1543FFD03492ED8C95A5DE525D` (break `/Game/Prototype1/Core/Structures/S_Character_Stats` (`self.Character_Stats`))) (`local.L_Index`) (`local.L_Attribute`))
  (return))

(fn `SetAttributeTotal`
  (params (Attribute :type "/Game/Prototype1/Core/Enum/Stat_Enum/E_Stat_AttributeList Enum" :default "NewEnumerator0") (DefaultValue :type "Float (double-precision)") (BonusValue :type "Float (double-precision)"))
  (returns (ReturnTotalValue :type "Float (double-precision)"))
  (locals (L_AttributeCurrent :type "/Game/Prototype1/Core/Enum/Stat_Enum/E_Stat_AttributeList Enum"))
  (bind _l_attributecurrent (`local.L_AttributeCurrent`))
  (bind _output_get (set `local.L_AttributeCurrent` Attribute))
  (switch `/Game/Prototype1/Core/Enum/Stat_Enum/E_Stat_AttributeList` _output_get
    (:`NewEnumerator0`
      (return (`local.DefaultValue`)))
    (:`NewEnumerator3`
      _)
    (:`NewEnumerator1`
      _)
    (:`NewEnumerator2`
      _)
    (:`NewEnumerator5`
      _)
    (:`NewEnumerator6`
      _)
    (:`NewEnumerator4`
      _)
    (:`NewEnumerator7`
      _))
  (bind _returnvalue (`self.GetAttributeDice` _l_attributecurrent))
  (return (`KismetMathLibrary.Conv_IntToDouble` (`KismetMathLibrary.FFloor` (+ _returnvalue (`self.GetAttributeValue` "NewEnumerator13" _l_attributecurrent) (* (+ (`local.DefaultValue`) (`local.BonusValue`)) 2.0))))))

(fn `SetStat`
  (params (Type :type "/Game/Prototype1/Core/Enum/Stat_Enum/E_Stat_Type Enum" :default "NewEnumerator0") (Stat :type "/Game/Prototype1/Core/Enum/Stat_Enum/E_Stat_List Enum" :default "NewEnumerator23") (Value :type "Float (double-precision)"))
  (locals (L_Stat :type "/Game/Prototype1/Core/Structures/Stats_Struc/S_SingleStat Structure") (L_StatRefIndex :type Integer :default 0))
  (bind (_resultstat _resultindex) (`self.GetStatRef` Stat))
  (bind _l_stat (`local.L_Stat`))
  (bind _l_stat_2 (`local.L_Stat`))
  (bind _l_stat_3 (`local.L_Stat`))
  (bind _l_stat_4 (`local.L_Stat`))
  (bind _l_stat_5 (`local.L_Stat`))
  (bind _l_stat_6 (`local.L_Stat`))
  (bind _l_stat_7 (`local.L_Stat`))
  (bind _l_stat_8 (`local.L_Stat`))
  (bind _l_stat_9 (`local.L_Stat`))
  (set `local.L_Stat` _resultstat)
  (set `local.L_StatRefIndex` _resultindex)
  (switch `/Game/Prototype1/Core/Enum/Stat_Enum/E_Stat_Type` (`local.Type`)
    (:`NewEnumerator0`
      (`KismetSystemLibrary.PrintString` "Warning: SetAttribute - \nError Can not use \"NONE\"")
      (return))
    (:`NewEnumerator1`
      (setmembers `/Game/Prototype1/Core/Structures/Stats_Struc/S_SingleStat` :`StructRef` _l_stat :`Current` (`KismetMathLibrary.FClamp` (`local.Value`) 0.0 (`.Final_26_B6CF407644F1FAECB10B66BCF3267972` (break `/Game/Prototype1/Core/Structures/Stats_Struc/S_SingleStat` _l_stat)))))
    (:`NewEnumerator5`
      (setmembers `/Game/Prototype1/Core/Structures/Stats_Struc/S_SingleStat` :`StructRef` _l_stat_2 :`Extra` (`KismetMathLibrary.FClamp` (`local.Value`) 0.0 (`.Final_26_B6CF407644F1FAECB10B66BCF3267972` (break `/Game/Prototype1/Core/Structures/Stats_Struc/S_SingleStat` _l_stat_2)))))
    (:`NewEnumerator2`
      (setmembers `/Game/Prototype1/Core/Structures/Stats_Struc/S_SingleStat` :`StructRef` _l_stat_3 :`Total` (`KismetMathLibrary.FClamp` (`local.Value`) 0.0 (`.Final_26_B6CF407644F1FAECB10B66BCF3267972` (break `/Game/Prototype1/Core/Structures/Stats_Struc/S_SingleStat` _l_stat_3)))))
    (:`NewEnumerator7`
      (setmembers `/Game/Prototype1/Core/Structures/Stats_Struc/S_SingleStat` :`StructRef` _l_stat_4 :`Final` (`KismetMathLibrary.FClamp` (`local.Value`) 0.0 (`.Final_26_B6CF407644F1FAECB10B66BCF3267972` (break `/Game/Prototype1/Core/Structures/Stats_Struc/S_SingleStat` _l_stat_4)))))
    (:`NewEnumerator8`
      (setmembers `/Game/Prototype1/Core/Structures/Stats_Struc/S_SingleStat` :`StructRef` _l_stat_5 :`Default` (`KismetMathLibrary.FClamp` (`local.Value`) 0.0 (`.Final_26_B6CF407644F1FAECB10B66BCF3267972` (break `/Game/Prototype1/Core/Structures/Stats_Struc/S_SingleStat` _l_stat_5)))))
    (:`NewEnumerator12`
      (setmembers `/Game/Prototype1/Core/Structures/Stats_Struc/S_SingleStat` :`StructRef` _l_stat_6 :`Power` (`KismetMathLibrary.FClamp` (`local.Value`) 0.0 (`.Final_26_B6CF407644F1FAECB10B66BCF3267972` (break `/Game/Prototype1/Core/Structures/Stats_Struc/S_SingleStat` _l_stat_6)))))
    (:`NewEnumerator10`
      (setmembers `/Game/Prototype1/Core/Structures/Stats_Struc/S_SingleStat` :`StructRef` _l_stat_7 :`Scale` (`KismetMathLibrary.FClamp` (`local.Value`) 0.0 (`.Final_26_B6CF407644F1FAECB10B66BCF3267972` (break `/Game/Prototype1/Core/Structures/Stats_Struc/S_SingleStat` _l_stat_7)))))
    (:`NewEnumerator13`
      (setmembers `/Game/Prototype1/Core/Structures/Stats_Struc/S_SingleStat` :`StructRef` _l_stat_8 :`Base` (`KismetMathLibrary.FClamp` (`local.Value`) 0.0 (`.Final_26_B6CF407644F1FAECB10B66BCF3267972` (break `/Game/Prototype1/Core/Structures/Stats_Struc/S_SingleStat` _l_stat_8)))))
    (:`NewEnumerator14`
      (setmembers `/Game/Prototype1/Core/Structures/Stats_Struc/S_SingleStat` :`StructRef` _l_stat_9 :`BaseMult` (`KismetMathLibrary.FClamp` (`local.Value`) 0.0 (`.Final_26_B6CF407644F1FAECB10B66BCF3267972` (break `/Game/Prototype1/Core/Structures/Stats_Struc/S_SingleStat` _l_stat_9))))))
  (`KismetArrayLibrary.Array_Set` (`.Stat_46_561705244D810CB8FD450891CBFE6803` (break `/Game/Prototype1/Core/Structures/S_Character_Stats` (`self.Character_Stats`))) (`local.L_StatRefIndex`) (`local.L_Stat`))
  (return))

(fn `SetStatScale`
  (params (Stat :type "/Game/Prototype1/Core/Enum/Stat_Enum/E_Stat_List Enum" :default "NewEnumerator23"))
  (returns (ReturnValue :type "Float (double-precision)"))
  (bind _returnvalue (`self.GetStatDice` Stat))
  (return (+ _returnvalue 0.0 (`self.GetStatDefault` Stat))))