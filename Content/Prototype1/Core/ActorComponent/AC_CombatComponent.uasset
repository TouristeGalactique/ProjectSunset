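; Actor component on BP_CharacterBase_Master that runs each unit's turn in an ATB-style battle, from initiative to victory or game over.
; A d20 plus Speed sets timer-based waits and delayed hero HUD display; ready units join a game-mode waiting list that pauses timers.
; Enemies pick random actions, heroes their chosen one; attacks move into melee, roll DataTable outcomes, apply damage and return.
; Only attack-type actions are implemented; others are placeholders.
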(event `self.ReceiveBeginPlay`
  (bind _asbp_character_base_master (cast `/Game/Prototype1/Core/Characters/BP_CharacterBase_Master` (`self.GetOwner`)))
  (bind _output_get (set `self.UnitCharacter` _asbp_character_base_master))
  (set `self.BattlePosition` (`Actor.GetTransform` _output_get))
  (`self.SetInitiative`))

(event `MoveToMeleePosition`
  (bind _unitcharacter (`self.UnitCharacter`))
  (bind _returnvalue (`Actor.K2_GetActorLocation` _unitcharacter))
  (bind _returnvalue_2 (`Actor.K2_GetActorLocation` (`self.CurrentTarget`)))
  (bind (_returnvalue_x _returnvalue_y) (`KismetMathLibrary.BreakVector` (`Actor.K2_GetActorLocation` (`self.UnitCharacter`))))
  (bind (_returnvalue_x_2 _returnvalue_y_2) (`KismetMathLibrary.BreakVector` (`Actor.K2_GetActorLocation` (`self.CurrentTarget`))))
  ;[0.004194 0.006619 0.02036 0.5] Enemy Mouvement
  (if (< _returnvalue_y _returnvalue_y_2)
    (set `self.MeleePoint` 100.0)
    (else
      (set `self.MeleePoint` -100.0)))
  (bind _returnvalue_3 (`KismetSystemLibrary.K2_SetTimerDelegate` (`|CreateDelegate` :!event `UpdateCamera`) 0.5))
  (set `self.UpdateCameraTimer` _returnvalue_3)
  (`KismetSystemLibrary.MoveComponentTo` (`Actor.RootComponent` _unitcharacter) (`KismetMathLibrary.MakeVector` (.x _returnvalue_2) (- (.y _returnvalue_2) (`self.MeleePoint`)) (.z _returnvalue)) (`KismetMathLibrary.FindLookAtRotation` _returnvalue _returnvalue_2) true true 1.0)
  (`self.SetAttackAction`))

(event `MoveBackToBattlePosition`
  (bind _returnvalue (`GameplayStatics.GetGameMode`))
  ;[0.004194 0.006619 0.02036 0.5] Enemy Mouvement
  ;;[0.004194 0.006619 0.02036 0.5] BackToBattlePosition
  (bind _returnmaincamera (message `/Game/Prototype1/Core/BPI_GameModeBattle.GetBattleCameraDefault` _returnvalue))
  (message `/Game/Prototype1/Core/BPI_GameModeBattle.SetBattleCamera` _returnvalue _returnmaincamera)
  (`KismetSystemLibrary.MoveComponentTo` (`Actor.RootComponent` (`self.UnitCharacter`)) (.location (`self.BattlePosition`)) (.rotation (`self.BattlePosition`)) true true 1.0)
  (`self.UnitTurnResult`))

(fn `AddToWaitingList`
  (message `/Game/Prototype1/Core/BPI_GameModeBattle.SetWaitingListUnit` (`GameplayStatics.GetGameMode`) (`self.UnitCharacter`))
  (return))

(fn `Debug_ShowInitDetails`
  (params (Name :type "Text (by ref)") (Dice :type Integer) (FinalValue :type "Float (double-precision)"))
  (bind _result (message `/Game/Prototype1/Core/BPI_GameModeBattle.GetBattleDebug` (`GameplayStatics.GetGameMode`)))
  (if (`.bBattle_InitDetails_24_26FEADAD46C06D7045AFC3A8908547EE` (break `/Game/Prototype1/Core/Structures/Setttings_Struc/BattleDebug` _result))
    (`KismetSystemLibrary.PrintString` (`KismetStringLibrary.Concat_StrStr` (`KismetTextLibrary.Conv_TextToString` Name) " Init: Dice: " (`KismetStringLibrary.Conv_IntToString` Dice) "  value: " (`KismetStringLibrary.Conv_DoubleToString` FinalValue)) true true (struct :`G` 0.66 :`B` 1.0 :`A` 1.0) 20.0)
    (return)
    (else
      (return))))

(fn `Debug_TurnPhase`
  (params (InText :type "Text (by ref)"))
  (bind _result (message `/Game/Prototype1/Core/BPI_GameModeBattle.GetBattleDebug` (`GameplayStatics.GetGameMode`)))
  (if (`.bBattle_ShowBattlePhase_19_0BBABD2B4FD1144E9EA6CF87BE532B38` (break `/Game/Prototype1/Core/Structures/Setttings_Struc/BattleDebug` _result))
    (`KismetSystemLibrary.PrintString` (`KismetStringLibrary.Concat_StrStr` (`KismetTextLibrary.Conv_TextToString` InText) " Start Waiting Turn") true true (struct :`G` 0.66 :`B` 1.0 :`A` 1.0) 5.0)
    (return)
    (else
      (return))))

(fn `GetRandomHero`
  (returns (TargetResult :type "/Game/Prototype1/Core/Characters/BP_CharacterBase_Master Object Reference"))
  (bind _returnvalue (`GameplayStatics.GetGameMode`))
  (message `/Game/Prototype1/Core/BPI_GameModeBattle.SetRandomTargetHero` _returnvalue)
  (bind _result (message `/Game/Prototype1/Core/BPI_GameModeBattle.GetRandomTargetHero` _returnvalue))
  (return _result))

(fn `SetActionResult`
  (returns (ActionResult :type "/Game/Prototype1/Core/Enum/Battle_Enum/E_Battle_ActionResult Enum"))
  (bind _returnvalue (`|GetDataTableRow` "/Game/Prototype1/Core/Structures/DT_BattleActionResult.DT_BattleActionResult" "Attack")
    (:`then`
      (bind _indexthatwon (`/Game/Prototype1/Core/FL_FunctionLibrary.SetProbability` (`.ActionResultProbabilities_7_02E023254C91E44404AF22AC63F9C45D` (break `/Game/Prototype1/Core/Structures/S_BattleActionResult` _returnvalue))))
      (return (`|GetArrayItem` (break `/Game/Prototype1/Core/Structures/S_BattleActionResult` _returnvalue) _indexthatwon)))))

(fn `SetAttackAction`
  (bind _actionresult (`self.SetActionResult`))
  (`KismetSystemLibrary.PrintString` (`|GetEnumeratorNameAsString` _actionresult))
  (switch `/Game/Prototype1/Core/Enum/Battle_Enum/E_Battle_ActionResult` _actionresult
    (:`NewEnumerator3`
      (`self.SetDamage`)
      ; Enemy Go Back in Waiting bar
      (`self.SetBackInLine` true)
      ; AttackAnimation
      (`self.SetAttackAnimation`)
      ; Unit Hit Animation
      (`/Game/Prototype1/Core/Characters/BP_CharacterBase_Master.SetHitAnimation` (`self.CurrentTarget`))
      (`self.SetAttackResolution`)
      (return))
    (:`NewEnumerator0`
      (`self.SetDamage`)
      ; Enemy Go Back in Waiting bar
      (`self.SetBackInLine` false)
      ; AttackAnimation
      (`self.SetAttackAnimation`)
      ; Unit Hit Animation
      (`/Game/Prototype1/Core/Characters/BP_CharacterBase_Master.SetHitAnimation` (`self.CurrentTarget`))
      (`self.SetAttackResolution`)
      (return))
    (:`NewEnumerator1`
      (set `self.Damage` 0)
      (`self.SetAttackResolution`)
      (return))
    (:`NewEnumerator2`
      (set `self.Damage` 0)
      ; AttackAnimation
      (`self.SetAttackAnimation`)
      ; Unit Dodge Animation
      (`/Game/Prototype1/Core/Characters/BP_CharacterBase_Master.SetDodgeAnimation` (`self.CurrentTarget`))
      (`self.SetAttackResolution`)
      (return))))

(fn `SetAttackAnimation`
  (bind _unitcharacter (`self.UnitCharacter`))
  (bind _location (.location (`SceneComponent.K2_GetComponentToWorld` (`/Game/Prototype1/Core/Characters/BP_CharacterBase_Master.SwordDummy` _unitcharacter))))
  ; Fait apparaitre l'épée
  (if (not (`/Game/Prototype1/Core/Characters/BP_CharacterBase_Master.bIsEnemy` _unitcharacter))
    (bind _returnvalue (`|SpawnActorFromClass` "/Game/Prototype1/Core/Characters/Weapon/BP_Sword.BP_Sword_C" (`KismetMathLibrary.MakeTransform` _location (`KismetMathLibrary.FindLookAtRotation` _location (`Actor.K2_GetActorLocation` (`self.CurrentTarget`))) (.scale (`SceneComponent.K2_GetComponentToWorld` (`/Game/Prototype1/Core/Characters/BP_CharacterBase_Master.SwordDummy` _unitcharacter)))) "Undefined" "MultiplyWithRoot" null null))
    (bind _output_get (set `self.Sword` _returnvalue))
    (`/Game/Prototype1/Core/Characters/Weapon/BP_Sword.sword strike` _output_get)
    (return)
    (else
      (return))))

(fn `SetAttackPreparation`
  (params (TargetUnit :type "/Game/Prototype1/Core/Characters/BP_CharacterBase_Master Object Reference") (ActionType :type "/Game/Prototype1/Core/Enum/E_ActionList Enum (by ref)"))
  (`self.ShowActionTxt` ActionType)
  (set `self.CurrentTarget` TargetUnit)
  (if (not (`/Game/Prototype1/Core/Characters/BP_CharacterBase_Master.bIsEnemy` (`self.UnitCharacter`)))
    (set `self.bHeroIsReady` false))
  (`self.SwitchUnitOrientation` false (`self.UnitCharacter`) (`self.CurrentTarget`))
  (`self.MoveToMeleePosition`)
  (return))

(fn `SetAttackResolution`
  (bind _damage (`self.Damage`))
  ; Show Unit Damage
  (`/Game/Prototype1/Core/Characters/BP_CharacterBase_Master.ShowUnitDamage` (`self.CurrentTarget`) _damage)
  ; Update HUD (if Hero)
  (`/Game/Prototype1/Core/Characters/BP_CharacterBase_Master.UpdateHeroData` (`self.CurrentTarget`) _damage)
  ; set new orientation *( if needed)
  (`self.SwitchUnitOrientation` true (`self.CurrentTarget`) (`self.UnitCharacter`))
  ; UpdateHP
  (`/Game/Prototype1/Core/Characters/BP_CharacterBase_Master.UpdateHealthPoints` (`self.CurrentTarget`) (`self.Damage`))
  ; Attack animation temporaty
  (bind _returnvalue (`KismetSystemLibrary.K2_SetTimerDelegate` (`|CreateDelegate` :!event `MoveBackToBattlePosition`) 1.0))
  (set `self.MoveBackToBattlePositionTimer` _returnvalue)
  (return))

(fn `SetBackInLine`
  (params (bIsCriticalSucceed :type Boolean))
  (return))

(fn `SetDamage`
  (returns (Damage :type Integer))
  ; Temporary calcul des damages ici
  (bind _output_get (set `self.Damage` (`.Attaque_11_356B32584BB4C604944AEBB342355F86` (break `/Game/Prototype1/Core/Structures/S_Character_Stats` (`/Game/Prototype1/Core/Characters/BP_CharacterBase_Master.CharacterStatsMain` (`self.UnitCharacter`))))))
  (return _output_get))

(fn `SetHeroActionSwitch`
  (params (Selection :type "/Game/Prototype1/Core/Enum/E_ActionList Enum" :default "NewEnumerator0") (TargetUnit :type "/Game/Prototype1/Core/Characters/BP_CharacterBase_Master Object Reference"))
  (switch `/Game/Prototype1/Core/Enum/E_ActionList` Selection
    (:`NewEnumerator0`
      _)
    (:`NewEnumerator3`
      ; Temporary
      (`self.UnitTurnResult` :!label _label)
      (return))
    (:`NewEnumerator5`
      (goto _label))
    (:`NewEnumerator4`
      (goto _label))
    (:`NewEnumerator1`
      (goto _label))
    (:`NewEnumerator2`
      (goto _label))
    (:`NewEnumerator6`
      (goto _label))
    (:`NewEnumerator7`
      _))
  (`self.SetAttackPreparation` TargetUnit Selection)
  (return))

(fn `SetInitiative`
  (returns (bIsCriticalSuccess :type Boolean))
  (locals (L_InitSuccess :type Integer :default 0))
  (bind ((`Name_18_28573E1C461470983A9F67A8EC7D0329` _name) (`Job_40_FBD99DE842F4748849277D9B871DA84D` _job) (`Speed_21_3FD34BBD45A9B2809ACB57BF48438D78` _speed)) (break `/Game/Prototype1/Core/Structures/S_Character_Stats` (`/Game/Prototype1/Core/Characters/BP_CharacterBase_Master.CharacterStatsMain` (`self.UnitCharacter`))))
  ; Initiative V4
  (bind _returnvalue (`/Game/Prototype1/Core/FL_FunctionLibrary.1D20`))
  (bind _returnvalue_2 (`KismetMathLibrary.MapRangeClamped` (+ _speed _returnvalue) 0.0 255.0 1.0 0.5))
  (set `self.SpeedModifier` _returnvalue_2)
  (bind _result (message `/Game/Prototype1/Core/BPI_GameModeBattle.GetBattleSettings` (`GameplayStatics.GetGameMode`)))
  (bind ((`WaitForActionTimeMax_21_2110F1934520F62BBC37A6BCED57A168` _waitforactiontimemax)) (break `/Game/Prototype1/Core/Structures/Setttings_Struc/S_BattleSettings` _result))
  (set `self.Wait for Action Time Max` _waitforactiontimemax)
  (bind _returnvalue_3 (== _returnvalue 20))
  (bind _output_get (set `self.bCriticalSuccess` _returnvalue_3))
  (bind _returnvalue_4 (`KismetMathLibrary.SelectFloat` (`self.Wait for Action Time Max`) (`KismetMathLibrary.SelectFloat` 0.0 (* (* _waitforactiontimemax _returnvalue_2) (`self.InitBonusMultiplicator`)) _returnvalue_3) (== _returnvalue 1)))
  (`self.Debug_ShowInitDetails` _name _returnvalue _returnvalue_4)
  (setmembers `/Game/Prototype1/Core/Structures/S_Character_Stats` :`StructRef` (`/Game/Prototype1/Core/Characters/BP_CharacterBase_Master.CharacterStatsMain` (`self.UnitCharacter`)) :`Initiative` _returnvalue_4)
  (set `self.Initiative Success` (select `int` _returnvalue :`0` "NewEnumerator2" :`1` "NewEnumerator2" :`2` "NewEnumerator1" :`3` "NewEnumerator1" :`4` "NewEnumerator1" :`5` "NewEnumerator1" :`6` "NewEnumerator1" :`7` "NewEnumerator1" :`8` "NewEnumerator1" :`9` "NewEnumerator1" :`10` "NewEnumerator1" :`11` "NewEnumerator1" :`12` "NewEnumerator1" :`13` "NewEnumerator1" :`14` "NewEnumerator1" :`15` "NewEnumerator1" :`16` "NewEnumerator1" :`17` "NewEnumerator1" :`18` "NewEnumerator1" :`19` "NewEnumerator1" :`20` "NewEnumerator0" :!type "/Game/Prototype1/Core/Enum/E_InitiativeSuccess Enum"))
  (return _output_get))

(fn `SetNewBattlePosition`
  (set `self.BattlePosition` (`Actor.GetTransform` (`self.UnitCharacter`)))
  (return))

(fn `SetNewInitiativeNextTurn`
  (if (`self.bCriticalSuccess`) :!label _label
    (bind _biscriticalsuccess (`self.SetInitiative`))
    (if _biscriticalsuccess
      (goto _label)
      (else
        (return)))
    (else
      (return))))

(fn `SetNextUnitSelectAction`
  (params (Index :type Integer))
  (bind _return (message `/Game/Prototype1/Core/BPI_GameModeBattle.GetWaitingListUnit` (`GameplayStatics.GetGameMode`)))
  (`self.SetUnitSelectAction` (`/Game/Prototype1/Core/Characters/BP_CharacterBase_Master.CombatComponent` (`|GetArrayItem` _return Index)))
  (return))

(fn `SetUnitNextTurn`
  (bind _returnvalue (`GameplayStatics.GetGameMode`))
  (bind _unitcharacter (`self.UnitCharacter`))
  (`KismetSystemLibrary.PrintString` (`KismetStringLibrary.Concat_StrStr` (`KismetSystemLibrary.GetDisplayName` (`self.UnitCharacter`)) " turn is Over") true true (struct :`G` 0.66 :`B` 1.0 :`A` 1.0) 10.0)
  (`self.SetNewInitiativeNextTurn`)
  (bind _return (message `/Game/Prototype1/Core/BPI_GameModeBattle.RemoveWaitingListIndex` _returnvalue 0))
  (if (`KismetArrayLibrary.Array_IsNotEmpty` _return)
    (`self.SetNextUnitSelectAction` 0)
    (`self.StartUnitWaitingTurn` _unitcharacter)
    (return)
    (else
      (message `/Game/Prototype1/Core/BPI_GameModeBattle.Unpause_StartUnitBattleTurnTimer` _returnvalue)
      (message `/Game/Prototype1/Core/BPI_GameModeBattle.Unpause_ShowHeroActionHUDTimer` _returnvalue)
      (`self.StartUnitWaitingTurn` _unitcharacter)
      (return))))

(fn `SetUnitSelectAction`
  (bind _unitcharacter (`self.UnitCharacter`))
  (bind ((`Name_18_28573E1C461470983A9F67A8EC7D0329` _name) (`Job_40_FBD99DE842F4748849277D9B871DA84D` _job) (`ActionList_30_5D04B8AA45490C3AC27FF8B3EEDA4587` _actionlist)) (break `/Game/Prototype1/Core/Structures/S_Character_Stats` (`/Game/Prototype1/Core/Characters/BP_CharacterBase_Master.CharacterStatsMain` _unitcharacter)))
  (if (not (`/Game/Prototype1/Core/Characters/BP_CharacterBase_Master.bIsEnemy` _unitcharacter))
    (`KismetSystemLibrary.PrintString` (`KismetStringLibrary.Concat_StrStr` "Hero Select Action : " (`KismetTextLibrary.Conv_TextToString` (`.Name_18_28573E1C461470983A9F67A8EC7D0329` (break `/Game/Prototype1/Core/Structures/S_Character_Stats` (`/Game/Prototype1/Core/Characters/BP_CharacterBase_Master.CharacterStatsMain` (`self.UnitCharacter`)))))))
    (message `/Game/Prototype1/Core/BPI_GameModeBattle.SetCurrentHero` (`GameplayStatics.GetGameMode`) (`self.UnitCharacter`))
    (bind _result (message `/Game/Prototype1/Core/BPI_GameModeBattle.GetEnemyUnits` (`GameplayStatics.GetGameMode`)))
    ; A verifier
    (if (== (`KismetArrayLibrary.Array_Find` _result (`self.CurrentTarget`)) -1)
      (set `self.CurrentTarget` (`|GetArrayItem` _result)))
    (set `/Game/Prototype1/Core/Characters/BP_CharacterBase_Master.RefenceUnit` (`self.UnitCharacter`) (`self.CurrentTarget`))
    (`self.SetHeroActionSwitch` (`self.Action Name`) (`self.CurrentTarget`))
    (return)
    (else
      (`KismetSystemLibrary.PrintString` (`KismetStringLibrary.Concat_StrStr` "Enemy Select Action :" (`KismetTextLibrary.Conv_TextToString` _name)))
      (`self.StartUnitAction` (`|GetArrayItem` _actionlist (`KismetMathLibrary.RandomIntegerInRange` 0 (`KismetArrayLibrary.Array_LastIndex` _actionlist))))
      (return))))

(fn `SetWaitingTimerDuration`
  (params (Initiative :type "Float (double-precision)"))
  (returns (DurationResult :type "Float (double-precision)") (ProgressAtStartResult :type "Float (double-precision)"))
  (if (`self.bIsFirstTurn`)
    (bind _output_get (set `self.WaitingTimerProgressAtStart` (`KismetMathLibrary.RandomFloatInRange` (`self.MinTimerStartValue`) Initiative)))
    (bind _output_get_2 (set `self.WaitingTimerDuration` (- Initiative _output_get)))
    (return _output_get_2 _output_get)
    (else
      (bind _output_get_3 (set `self.WaitingTimerProgressAtStart` 0.0))
      (bind _output_get_4 (set `self.WaitingTimerDuration` (* (`self.Wait for Action Time Max`) (`self.SpeedModifier`))))
      (return _output_get_4 _output_get_3))))

(fn `ShowActionTxt`
  (params (InputPin :type "/Game/Prototype1/Core/Enum/E_ActionList Enum (by ref)"))
  (bind _result (message `/Game/Prototype1/Core/BPI_GameModeBattle.GetBattleHUD` (`GameplayStatics.GetGameMode`)))
  (`/Game/Prototype1/CommonUI/Widgets/Battle_Widget/WBP_BattleMainHUD.SetDisplayActionText` _result (`self.UnitCharacter`) InputPin)
  (return))

(fn `ShowHeroActionHUD`
  (bind _unitcharacter (`self.UnitCharacter`))
  (if (not (`/Game/Prototype1/Core/Characters/BP_CharacterBase_Master.bIsEnemy` (`self.UnitCharacter`)))
    (`/Game/Prototype1/Core/Characters/BP_CharacterBase_Master.ShowUnitActionHUD` _unitcharacter)
    (`/Game/Prototype1/Core/Characters/BP_CharacterBase_Master.ShowHeroPointer` _unitcharacter true)
    (message `/Game/Prototype1/Core/BPI_BattlePlayerController.SetBackBtnIsActivated` (`GameplayStatics.GetPlayerController` 0) true)
    (return)
    (else
      (return))))

(fn `StartUnitAction`
  (params (UnitAction :type "/Game/Prototype1/Core/Enum/E_ActionList Enum" :default "NewEnumerator0"))
  (switch `/Game/Prototype1/Core/Enum/E_ActionList` UnitAction
    (:`NewEnumerator0`
      (bind _targetresult (`self.GetRandomHero`))
      (`self.SetAttackPreparation` _targetresult UnitAction)
      (set `/Game/Prototype1/Core/Characters/BP_CharacterBase_Master.RefenceUnit` (`self.UnitCharacter`) (`self.CurrentTarget`))
      (return))
    (:`NewEnumerator1`
      (return))
    (:`NewEnumerator2`
      (return))))

(fn `StartUnitBattleTurn`
  (bind _returnvalue (`GameplayStatics.GetGameMode`))
  (if (`/Game/Prototype1/Core/Characters/BP_CharacterBase_Master.bIsEnemy` (`self.UnitCharacter`))
    _
    (elif (`self.bHeroIsReady`)
      _
      (else
        (return))))
  (`self.AddToWaitingList`)
  (message `/Game/Prototype1/Core/BPI_GameModeBattle.Pause_StartUnitBattleTurnTimer` _returnvalue)
  (message `/Game/Prototype1/Core/BPI_GameModeBattle.Pause_ShowHeroActionHUDTimer` _returnvalue)
  (`self.SetNextUnitSelectAction` 0)
  (return))

(fn `StartUnitWaitingTurn`
  (params (Unit :type "/Game/Prototype1/Core/Characters/BP_CharacterBase_Master Object Reference"))
  (bind _waitingtimerduration (`self.WaitingTimerDuration`))
  (bind ((`Name_18_28573E1C461470983A9F67A8EC7D0329` _name) (`Job_40_FBD99DE842F4748849277D9B871DA84D` _job) (`Initiative_22_E9CE061F40F492CAB4B6F6A0ADCC0FA8` _initiative)) (break `/Game/Prototype1/Core/Structures/S_Character_Stats` (`/Game/Prototype1/Core/Characters/BP_CharacterBase_Master.CharacterStatsMain` Unit)))
  (bind ((`Job_40_FBD99DE842F4748849277D9B871DA84D` _job_2) (`Initiative_22_E9CE061F40F492CAB4B6F6A0ADCC0FA8` _initiative_2)) (break `/Game/Prototype1/Core/Structures/S_Character_Stats` (`/Game/Prototype1/Core/Characters/BP_CharacterBase_Master.CharacterStatsMain` (`self.UnitCharacter`))))
  (bind _returnvalue (- _initiative_2 (* _initiative_2 (/ (`self.ChoosingTimePercent`) 100.0))))
  (`self.Debug_TurnPhase` _name)
  (switch `/Game/Prototype1/Core/Enum/E_InitiativeSuccess` (`self.Initiative Success`)
    (:`NewEnumerator0`
      (set `self.WaitingTimerDuration` 0.05))
    (:`NewEnumerator1`
      (`self.SetWaitingTimerDuration` _initiative))
    (:`NewEnumerator2`
      (set `self.WaitingTimerProgressAtStart` 0.0)
      (set `self.WaitingTimerDuration` (`self.Wait for Action Time Max`))))
  (bind _returnvalue_2 (`KismetSystemLibrary.K2_SetTimerDelegate` (`|CreateDelegate` :!event `StartUnitBattleTurn`) (`self.WaitingTimerDuration`)))
  (set `self.StartUnitBattleTurnTimer` _returnvalue_2)
  (set `self.bIsFirstTurn` false)
  ;[0.004194 0.006619 0.02036 0.5] Affiche HUD Action si Hero
  (if (>= _returnvalue _waitingtimerduration)
    (`self.ShowHeroActionHUD`)
    (return)
    (else
      (bind _returnvalue_3 (`KismetSystemLibrary.K2_SetTimerDelegate` (`|CreateDelegate` :!event `ShowHeroActionHUD`) (- _waitingtimerduration _returnvalue)))
      (set `self.ShowHeroActionHUDTimer` _returnvalue_3)
      (return))))

(fn `SwitchUnitOrientation`
  (params (bSwitchTargetInstead :type Boolean) (TargetToSwitch :type "/Game/Prototype1/Core/Characters/BP_CharacterBase_Master Object Reference") (Reference :type "/Game/Prototype1/Core/Characters/BP_CharacterBase_Master Object Reference"))
  (bind (_returnvalue_x _returnvalue_y) (`KismetMathLibrary.BreakVector` (`Actor.GetActorForwardVector` TargetToSwitch)))
  (bind (_returnvalue_x_2 _returnvalue_y_2) (`KismetMathLibrary.BreakVector` (- (`Actor.K2_GetActorLocation` TargetToSwitch) (`Actor.K2_GetActorLocation` Reference))))
  (if (not (== (`KismetMathLibrary.SignOfFloat` _returnvalue_y) (* (`KismetMathLibrary.SignOfFloat` _returnvalue_y_2) -1.0)))
    (`/Game/Prototype1/Core/FL_FunctionLibrary.SetUnitOrientation` TargetToSwitch true)
    (`self.SetNewBattlePosition` (`/Game/Prototype1/Core/Characters/BP_CharacterBase_Master.CombatComponent` TargetToSwitch))
    (return)
    (else
      (return))))

(fn `UnitTurnResult`
  (bind _returnvalue (`GameplayStatics.GetGameMode`))
  (bind _returnvalue_2 (`GameplayStatics.GetGameMode`))
  (bind _result (message `/Game/Prototype1/Core/BPI_GameModeBattle.GetBattleResult` (`GameplayStatics.GetGameMode`)))
  (switch `/Game/Prototype1/Core/Enum/Battle_Enum/E_Battle_TurnResult` _result
    (:`NewEnumerator0`
      ; Il y a encore des Enemis et des heros
      (`self.SetUnitNextTurn`)
      (return))
    (:`NewEnumerator1`
      ; Victory
      (bind _result_2 (message `/Game/Prototype1/Core/BPI_GameModeBattle.GetEndingMenuOnScreen` _returnvalue))
      (if (not _result_2)
        (message `/Game/Prototype1/Core/BPI_GameModeBattle.SetEndingMenuOnScreen` _returnvalue true)
        (bind _result_3 (message `/Game/Prototype1/Core/BPI_GameModeBattle.GetBattleHUD` (`GameplayStatics.GetGameMode`)))
        (`/Game/Prototype1/CommonUI/Widgets/Battle_Widget/WBP_BattleMainHUD.PushEndingMenu` _result_3)
        (return)
        (else
          (return))))
    (:`NewEnumerator2`
      ; Game over
      (bind _result_4 (message `/Game/Prototype1/Core/BPI_GameModeBattle.GetEndingMenuOnScreen` _returnvalue_2))
      (if (not _result_4)
        (message `/Game/Prototype1/Core/BPI_GameModeBattle.SetEndingMenuOnScreen` _returnvalue_2 true)
        (`KismetSystemLibrary.PrintString` "Game Over")
        (bind _result_5 (message `/Game/Prototype1/Core/BPI_GameModeBattle.GetBattleHUD` (`GameplayStatics.GetGameMode`)))
        (`/Game/Prototype1/CommonUI/Widgets/Battle_Widget/WBP_BattleMainHUD.PushGameOver` _result_5)
        (return)
        (else
          (return))))))

(fn `UpdateCamera`
  (message `/Game/Prototype1/Core/BPI_GameModeBattle.SetBattleCamera` (`GameplayStatics.GetGameMode`) (`self.UnitCharacter`))
  (return))