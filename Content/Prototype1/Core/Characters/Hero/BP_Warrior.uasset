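; BP_Warrior is the Warrior hero character Blueprint, which shows its character info when play begins.
; After the parent BeginPlay and a short delay, it calls a chain of Show functions for name and level, stats, XP, HP, MP, attack and defense.
; The graph defines none of these functions, and Tick and the construction script add no logic of their own.
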(event `self.ReceiveBeginPlay`
  (`parent.ReceiveBeginPlay`)
  (`KismetSystemLibrary.Delay` 0.2)
  (`self.ShowNameLv`)
  (`self.ShowStats`)
  (`self.Show XP`)
  (`self.Show HP`)
  (`self.ShowMp`)
  (`self.ShowAtk`)
  (`self.ShowDef`))

(event `self.ReceiveTick`
  (params (DeltaSeconds :type "Float (single-precision)")))

(fn `UserConstructionScript`
  (`parent.UserConstructionScript`))