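; BP_Character_Master is a character Blueprint that holds combat stats in a CharacterStats struct: HP, MP, their maximums, initiative, attack and speed.
; SetCharacterStats fills the struct from its inputs.
; SetInitiative rolls initiative as Speed plus the result of a 1D20 call and writes it back into the struct.
; An unconnected EventGraph fragment would destroy the actor at zero HP, but it never runs.
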(fn `SetCharacterStats`
  (params (`Character Stats HP` :type Integer) (`Character Stats HP Max` :type Integer) (`Character Stats MP` :type Integer) (`Character Stats MP Max` :type Integer) (`Character Stats Initiative` :type Integer) (`Character Stats Attaque` :type Integer) (`Character Stats Speed` :type Integer))
  (set `self.CharacterStats` (make `/Game/Prototype1/Core/Structures/S_Character_Stat` `Character Stats HP` `Character Stats HP Max` `Character Stats MP` `Character Stats MP Max` `Character Stats Initiative` `Character Stats Attaque` `Character Stats Speed`))
  (return))

(fn `SetInitiative`
  (bind (_characterstats_hp _characterstats_hp_max _characterstats_mp _characterstats_mp_max _characterstats_initiative _characterstats_attaque _characterstats_speed) (break `/Game/Prototype1/Core/Structures/S_Character_Stat` (`self.CharacterStats`)))
  (setmembers `/Game/Prototype1/Core/Structures/S_Character_Stat` :`StructRef` (`self.CharacterStats`) :`Initiative` (+ _characterstats_speed (`/Game/Prototype1/Core/FL_FunctionLibrary.1D20`)))
  (return))

(fn `UserConstructionScript`)