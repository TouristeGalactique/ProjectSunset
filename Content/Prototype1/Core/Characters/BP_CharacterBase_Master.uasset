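; Base character Blueprint for battle units, holding a stats struct and handling health, attacks, facing and the battle command HUD.
; Attack passes the attacker's Attaque stat as an additive delta to the target's UpdateHealthPoints, which caps at max HP and destroys the actor at zero or below.
; Helpers create and remove the BattleActionCommands widget, and negate the target's capsule yaw when it equals the attacker's.
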(fn `Attack`
  (params (TargetUnit :type "/Game/Prototype1/Core/Characters/BP_CharacterBase_Master Object Reference"))
  (bind _newhealthpoints (`self.UpdateHealthPoints` TargetUnit (`.Attaque_11_356B32584BB4C604944AEBB342355F86` (break `/Game/Prototype1/Core/Structures/S_Character_Stats` (`self.CharacterStatsMain`)))))
  (`KismetSystemLibrary.PrintString` (`KismetStringLibrary.Conv_IntToString` _newhealthpoints) true true (struct :`G` 0.66 :`B` 1.0 :`A` 1.0) 20.0)
  (return))

(fn `DestroyBattleActionHUD`
  (`Widget.RemoveFromParent` (`self.BattleActionCommand`))
  (return))

(fn `isUnitFaceOpponent`
  (params (AttackerUnit :type "/Game/Prototype1/Core/Characters/BP_CharacterBase_Master Object Reference") (TargetUnit :type "/Game/Prototype1/Core/Characters/BP_CharacterBase_Master Object Reference"))
  (returns (ReturnValue :type Boolean))
  (return (== (.yaw (`SceneComponent.K2_GetComponentRotation` (`Character.CapsuleComponent` AttackerUnit))) (.yaw (`SceneComponent.K2_GetComponentRotation` (`Character.CapsuleComponent` TargetUnit))))))

(fn `SetCharacterStats`
  (params (`Character Stats Name` :type Text) (`Character Stats HP` :type Integer) (`Character Stats HP Max` :type Integer) (`Character Stats MP` :type Integer) (`Character Stats MP Max` :type Integer) (`Character Stats Initiative` :type "Float (double-precision)") (`Character Stats Attaque` :type Integer) (`Character Stats Speed` :type "Float (double-precision)"))
  (set `self.CharacterStatsMain` (make `/Game/Prototype1/Core/Structures/S_Character_Stats` `Character Stats Name` `Character Stats HP` `Character Stats HP Max` `Character Stats MP` `Character Stats MP Max` `Character Stats Initiative` `Character Stats Attaque` `Character Stats Speed`))
  (return))

(fn `SetUnitFaceOpponent`
  (params (AttackerUnit :type "/Game/Prototype1/Core/Characters/BP_CharacterBase_Master Object Reference") (TargetUnit :type "/Game/Prototype1/Core/Characters/BP_CharacterBase_Master Object Reference"))
  (bind _capsulecomponent (`Character.CapsuleComponent` TargetUnit))
  (bind _roll (.roll (`SceneComponent.K2_GetComponentRotation` _capsulecomponent)))
  (bind _pitch (.pitch (`SceneComponent.K2_GetComponentRotation` _capsulecomponent)))
  (bind _yaw (.yaw (`SceneComponent.K2_GetComponentRotation` _capsulecomponent)))
  (bind _returnvalue (`self.isUnitFaceOpponent` AttackerUnit TargetUnit))
  (if _returnvalue
    (`SceneComponent.K2_SetWorldRotation` _capsulecomponent (`KismetMathLibrary.MakeRotator` _roll _pitch (* _yaw -1.0)) false false)
    (return)
    (else
      (`SceneComponent.K2_SetWorldRotation` _capsulecomponent (`KismetMathLibrary.MakeRotator` _roll _pitch _yaw) false false)
      (return))))

(fn `ShowBattleActionHUD`
  (params (Unit :type "/Game/Prototype1/Core/Characters/BP_CharacterBase_Master Object Reference"))
  (bind _returnvalue (`|CreateWidget` "/Game/Prototype1/HUD/Widgets/BattleActionCommands.BattleActionCommands_C" null Unit))
  (bind _output_get (set `self.BattleActionCommand` _returnvalue))
  (`UserWidget.AddToViewport` _output_get 0)
  (return))

(fn `UpdateHealthPoints`
  (params (Delta :type Integer))
  (returns (NewHealthPoints :type Integer))
  (bind _characterstatsmain (`self.CharacterStatsMain`))
  (bind (_name _hp_current _hp_max) (break `/Game/Prototype1/Core/Structures/S_Character_Stats` (`self.CharacterStatsMain`)))
  (bind (_name_2 _hp_current_2 _hp_max_2) (break `/Game/Prototype1/Core/Structures/S_Character_Stats` _characterstatsmain))
  (bind _returnvalue (+ Delta _hp_current))
  ;[0.004194 0.006619 0.02036 0.5] Updater les points de vie du Character
  ;;[0.004194 0.006619 0.02036 0.5] Si New HP > HP max
  (if (< _returnvalue _hp_max)
    (setmembers `/Game/Prototype1/Core/Structures/S_Character_Stats` :`StructRef` (`self.CharacterStatsMain`) :`HP_Current` _returnvalue)
    (`self.UpdateIsDead`)
    (return _returnvalue)
    (else
      (setmembers `/Game/Prototype1/Core/Structures/S_Character_Stats` :`StructRef` _characterstatsmain :`HP_Current` _hp_max_2)
      (return _hp_max_2))))

(fn `UpdateIsDead`
  ;[0.004194 0.006619 0.02036 0.5] Vérifie si le character n'a plus de point de vie
  (if (<= (`.HP_Current_19_A6E8770C475F8996C13A769BC42463EB` (break `/Game/Prototype1/Core/Structures/S_Character_Stats` (`self.CharacterStatsMain`))) 0)
    (set `self.IsDead` true)
    (`self.K2_DestroyActor`)
    (return)
    (else
      (set `self.IsDead` false)
      (return))))

(fn `UserConstructionScript`)