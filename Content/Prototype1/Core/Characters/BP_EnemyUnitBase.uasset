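; Base Blueprint for enemy units in the prototype, layered on a parent unit class that supplies the attack logic.
; Most overrides only call the parent; the attack move also turns the unit toward its target and saves its position.
; It then jumps to a location derived from the target's capsule, with X and Y scaled, and starts a short timer.
; TemporaryBackAnimation restores the saved position without interpolation, as a placeholder return move.
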(event `self.ReceiveBeginPlay`
  (`parent.ReceiveBeginPlay`))

(fn `Attack`
  (params (TargetUnit :type "/Game/Prototype1/Core/Characters/BP_CharacterBase_Master Object Reference") (bIsCounterAttack :type Boolean))
  (`parent.Attack` TargetUnit bIsCounterAttack)
  (return))

(fn `StartAttackAnimation`
  (params (TargetUnit :type "/Game/Prototype1/Core/Characters/BP_CharacterBase_Master Object Reference"))
  (`parent.StartAttackAnimation` TargetUnit)
  (return))

(fn `StartAttackerMoveBackAnimation`
  (`parent.StartAttackerMoveBackAnimation`)
  (return))

(fn `StartAttackMoveAnimation`
  (params (TargetUnit :type "/Game/Prototype1/Core/Characters/BP_CharacterBase_Master Object Reference"))
  (bind (_returnvalue_x _returnvalue_y _returnvalue_z) (`KismetMathLibrary.BreakVector` (`SceneComponent.K2_GetComponentLocation` (`Character.CapsuleComponent` TargetUnit))))
  (`parent.StartAttackMoveAnimation` TargetUnit)
  (`self.SetUnitFaceOpponent` TargetUnit self)
  (set `self.UnitBasePosition` (`SceneComponent.K2_GetComponentLocation` (`self.CapsuleComponent`)))
  (`self.K2_SetActorRelativeLocation` self (`KismetMathLibrary.MakeVector` (* _returnvalue_x 4.0) (* _returnvalue_y 4.0) _returnvalue_z) false false)
  (`KismetSystemLibrary.K2_SetTimerDelegate` (`|CreateDelegate` :!event `TemporaryBackAnimation`) 2.0)
  (return))

(fn `TemporaryBackAnimation`
  (`self.K2_SetActorRelativeLocation` self (`self.UnitBasePosition`) false false)
  (return))

(fn `UserConstructionScript`
  (`parent.UserConstructionScript`))