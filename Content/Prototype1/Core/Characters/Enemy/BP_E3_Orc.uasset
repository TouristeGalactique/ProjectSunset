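; BP_E3_Orc is an Orc enemy Blueprint that extends a parent enemy class with its own startup and death fade.
; Shortly after BeginPlay it calls SHowXpDrop.
; DeathAnimation calls the parent version, swaps the Arm, Arm1 and Stomac meshes to a death material and starts a fast looping timer.
; SetDeathOpacity steps DeathTimeMultiplier down and pushes it to those materials as a scalar parameter.
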(event `self.ReceiveBeginPlay`
  (`parent.ReceiveBeginPlay`)
  (`KismetSystemLibrary.Delay` 0.2)
  (`self.SHowXpDrop`))

(fn `DeathAnimation`
  (`parent.DeathAnimation`)
  (`PrimitiveComponent.SetMaterial` (`self.Arm`) 0 "/Game/Prototype1/Materials/EnemyDeath_Inst.EnemyDeath_Inst")
  (`PrimitiveComponent.SetMaterial` (`self.Arm1`) 0 "/Game/Prototype1/Materials/EnemyDeath_Inst.EnemyDeath_Inst")
  (`PrimitiveComponent.SetMaterial` (`self.Stomac`) 0 "/Game/Prototype1/Materials/EnemyDeath_Inst.EnemyDeath_Inst")
  (bind _returnvalue (`KismetSystemLibrary.K2_SetTimerDelegate` (`|CreateDelegate` :!event `SetDeathOpacity`) 0.001 true true))
  (set `self.SetDeathOpacityTimer` _returnvalue))

(fn `SetDeathOpacity`
  (`parent.SetDeathOpacity`)
  (bind _output_get (set `self.DeathTimeMultiplier` (+ (`self.DeathTimeMultiplier`) -0.01)))
  (`MeshComponent.SetScalarParameterValueOnMaterials` (`self.Arm`) "DeathTimeMultiplier" _output_get)
  (`MeshComponent.SetScalarParameterValueOnMaterials` (`self.Arm1`) "DeathTimeMultiplier" _output_get)
  (`MeshComponent.SetScalarParameterValueOnMaterials` (`self.Stomac`) "DeathTimeMultiplier" _output_get)
  (return))

(fn `UserConstructionScript`
  (`parent.UserConstructionScript`))