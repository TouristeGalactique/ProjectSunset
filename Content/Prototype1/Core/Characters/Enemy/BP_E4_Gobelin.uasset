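; Goblin enemy Blueprint that extends a parent enemy class, adding death-fade visuals for its two ear meshes.
; DeathAnimation calls the parent, swaps both ears to a death material instance and starts a fast looping timer stored as SetDeathOpacityTimer.
; SetDeathOpacity calls the parent, then decrements DeathTimeMultiplier and pushes it to the ear materials as a scalar parameter.
; BeginPlay only calls the parent; the stat-display calls are unconnected.
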(event `self.ReceiveBeginPlay`
  (`parent.ReceiveBeginPlay`))

(fn `DeathAnimation`
  (`parent.DeathAnimation`)
  (`PrimitiveComponent.SetMaterial` (`self.OreilleDr`) 0 "/Game/Prototype1/Materials/EnemyDeath_Inst.EnemyDeath_Inst")
  (`PrimitiveComponent.SetMaterial` (`self.OreilleL`) 0 "/Game/Prototype1/Materials/EnemyDeath_Inst.EnemyDeath_Inst")
  (bind _returnvalue (`KismetSystemLibrary.K2_SetTimerDelegate` (`|CreateDelegate` :!event `SetDeathOpacity`) 0.001 true true))
  (set `self.SetDeathOpacityTimer` _returnvalue)
  (return))

(fn `SetDeathOpacity`
  (`parent.SetDeathOpacity`)
  (bind _output_get (set `self.DeathTimeMultiplier` (+ (`self.DeathTimeMultiplier`) -0.01)))
  (`MeshComponent.SetScalarParameterValueOnMaterials` (`self.OreilleDr`) "DeathTimeMultiplier" _output_get)
  (`MeshComponent.SetScalarParameterValueOnMaterials` (`self.OreilleL`) "DeathTimeMultiplier" _output_get)
  (return))

(fn `UserConstructionScript`
  (`parent.UserConstructionScript`))