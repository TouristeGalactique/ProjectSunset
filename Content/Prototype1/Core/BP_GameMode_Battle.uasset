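; Battle game mode that sets up a turn-based fight with a top-down camera, spawned units and a battle HUD.
; Enemy count comes from a d6 roll while ally count is fixed at one; each count selects a random formation, filling matching spawners and destroying the rest.
; Units queue through TurnRequest, and a DoOnce gate admits one turn at a time, with ReadyNextTurn resetting it.
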(event `verificator`
  (`KismetSystemLibrary.PrintString` (`KismetStringLibrary.Concat_StrStr` "Enemy Number = " (`KismetStringLibrary.Conv_IntToString` (`self.Enemy Per Battle`))) true true (struct :`G` 0.66 :`B` 1.0 :`A` 1.0) 20.0))

(event `self.ReceiveBeginPlay`
  (`parent.ReceiveBeginPlay`)
  ;[0.004194 0.006619 0.02036 0.5] Set enemy list et PartyUnits list
  (`self.SetPartyUnitList`)
  (`self.SetPartyEnemyList`)
  (`self.SetMainBattleCamera`)
  (`self.SetSpawnerTypeList`)
  ;[0.004194 0.006619 0.02036 0.5] Enemy Set up
  (`self.SetBattleEnemyNumber`)
  (`self.verificator`)
  (`self.SetEnemyFormation`)
  ;[0.004194 0.006619 0.02036 0.5] Ally Set up
  (`self.SetBattleAllyNumber`)
  (`self.SetAllyFormation`)
  (`self.SetAllUnits`)
  (`self.SetBattleHUD`))

(event `TurnRequest`
  (params (Unit :type "/Game/Prototype1/Core/Characters/BP_CharacterBase_Master Object Reference"))
  ;[0.004194 0.006619 0.02036 0.5] Ajout Unit au TurnOrder
  (`KismetArrayLibrary.Array_AddUnique` (`self.TurnOrder`) Unit)
  (`self.StartTurn`))

(event `StartTurn`
  (bind _combatcomponent (`/Game/Prototype1/Core/Characters/BP_CharacterBase_Master.CombatComponent` (`|GetArrayItem` (`self.TurnOrder`))))
  ;[0.004194 0.006619 0.02036 0.5] Détermine le tour de jeu du Unit
  (`/Engine/EditorBlueprintResources/StandardMacros.DoOnce` false :!label _label
    (:`Completed`
      (if (`KismetArrayLibrary.Array_IsValidIndex` (`self.TurnOrder`))
        (`/Game/Prototype1/Core/CombatComponent.StartUnitTurn` _combatcomponent)
        (add `/Game/Prototype1/Core/CombatComponent.TurnEnded` _combatcomponent (`|CreateDelegate` :!event `ReadyNextTurn`))
        ;[0.004194 0.006619 0.02036 0.5] Enlève la Unit du Turn Order
        (`KismetArrayLibrary.Array_Remove` (`self.TurnOrder`))
        (else
          (`self.ReadyNextTurn`))))))

(event `ReadyNextTurn`
  ;[0.004194 0.006619 0.02036 0.5] Détermine le tour de jeu du Unit
  (`|ExecutionSequence`
    (:`then_0`
      (goto _label :!via `Reset`))
    (:`then_1`
      (if (`KismetArrayLibrary.Array_IsValidIndex` (`self.TurnOrder`))
        (`self.StartTurn`)))))

(fn `SetAllUnits`
  (bind _outactors (`GameplayStatics.GetAllActorsOfClass` "/Game/Prototype1/Core/Characters/BP_PartyUnitBase.BP_PartyUnitBase_C"))
  (set `self.PartyUnits` _outactors)
  (bind _outactors_2 (`GameplayStatics.GetAllActorsOfClass` "/Game/Prototype1/Core/Characters/BP_EnemyUnitBase.BP_EnemyUnitBase_C"))
  (set `self.EnemyUnits` _outactors_2))

(fn `SetAllyFormation`
  (bind _allyspawnerlist (`self.AllySpawnerList`))
  (switch `int` (`self.Ally Per Battle`)
    (:`1`
      (`self.SpawnCharacterInFormation` (`|MakeArray` "NewEnumerator19" :!type "/Game/Prototype1/Core/Enum/E_Formation Enum") _allyspawnerlist))
    (:`2`
      (`self.SpawnCharacterInFormation` (`|MakeArray` "NewEnumerator21" :!type "/Game/Prototype1/Core/Enum/E_Formation Enum") _allyspawnerlist))
    (:`3`
      (`self.SpawnCharacterInFormation` (`|MakeArray` "NewEnumerator22" :!type "/Game/Prototype1/Core/Enum/E_Formation Enum") _allyspawnerlist))
    (:`4`
      (`self.SpawnCharacterInFormation` (`|MakeArray` "NewEnumerator23" :!type "/Game/Prototype1/Core/Enum/E_Formation Enum") _allyspawnerlist)))
  (return))

(fn `SetBattleAllyNumber`
  (`/Game/Prototype1/Core/FL_FunctionLibrary.1D4`)
  (set `self.Ally Per Battle` 1)
  (return))

(fn `SetBattleEnemyNumber`
  (bind _returnvalue (`/Game/Prototype1/Core/FL_FunctionLibrary.1D6`))
  (set `self.Enemy Per Battle` _returnvalue)
  (return))

(fn `SetBattleHUD`
  (bind _returnvalue (`|CreateWidget` "/Game/Prototype1/HUD/Widgets/BattleHeadSUpDisplay.BattleHeadSUpDisplay_C"))
  (bind _output_get (set `self.BattleHUD` _returnvalue))
  (`UserWidget.AddToViewport` _output_get 0)
  (for _array_element (`self.PartyUnits`)
    (`/Game/Prototype1/HUD/Widgets/BattleHeadSUpDisplay.AddPartyUnitToHUD` (`self.BattleHUD`) _array_element))
  (return))

(fn `SetEnemyFormation`
  (switch `int` (`self.Enemy Per Battle`)
    (:`1`
      (`self.SpawnCharacterInFormation` (`|MakeArray` "NewEnumerator1" "NewEnumerator2" :!type "/Game/Prototype1/Core/Enum/E_Formation Enum") (`self.EnemySpawnerList`)))
    (:`2`
      (`self.SpawnCharacterInFormation` (`|MakeArray` "NewEnumerator3" "NewEnumerator4" :!type "/Game/Prototype1/Core/Enum/E_Formation Enum") (`self.EnemySpawnerList`)))
    (:`3`
      (`self.SpawnCharacterInFormation` (`|MakeArray` "NewEnumerator5" "NewEnumerator6" "NewEnumerator7" :!type "/Game/Prototype1/Core/Enum/E_Formation Enum") (`self.EnemySpawnerList`)))
    (:`4`
      (`self.SpawnCharacterInFormation` (`|MakeArray` "NewEnumerator8" "NewEnumerator9" "NewEnumerator10" :!type "/Game/Prototype1/Core/Enum/E_Formation Enum") (`self.EnemySpawnerList`)))
    (:`5`
      (`self.SpawnCharacterInFormation` (`|MakeArray` "NewEnumerator11" "NewEnumerator12" "NewEnumerator13" "NewEnumerator14" "NewEnumerator15" :!type "/Game/Prototype1/Core/Enum/E_Formation Enum") (`self.EnemySpawnerList`)))
    (:`6`
      (`self.SpawnCharacterInFormation` (`|MakeArray` "NewEnumerator16" "NewEnumerator17" "NewEnumerator18" :!type "/Game/Prototype1/Core/Enum/E_Formation Enum") (`self.EnemySpawnerList`))))
  (return))

(fn `SetMainBattleCamera`
  (bind _returnvalue (`GameplayStatics.GetActorOfClass` "/Game/Prototype1/Core/Cameras/BP_Camera_Battle_TopDown.BP_Camera_Battle_TopDown_C"))
  (bind _output_get (set `self.MainBattleCamera` _returnvalue))
  (`PlayerController.SetViewTargetWithBlend` (`GameplayStatics.GetPlayerController` 0) _output_get 0.0 "VTBlend_Linear" 0.0 false)
  (return))

(fn `SetPartyEnemyList`
  (set `self.EnemyCharacterList` (`self.EnemyCharacterList`))
  (return))

(fn `SetPartyUnitList`
  (set `self.PartyUnitCharacterList` (`self.PartyUnitCharacterList`))
  (return))

(fn `SetSpawnerTypeList`
  (bind _outactors (`GameplayStatics.GetAllActorsOfClass` "/Game/Prototype1/Core/Characters/BP_CharacterSpawner.BP_CharacterSpawner_C"))
  (for _array_element _outactors
    (if (`/Game/Prototype1/Core/Characters/BP_CharacterSpawner.IsEnemy` _array_element)
      (`KismetArrayLibrary.Array_Add` (`self.EnemySpawnerList`) _array_element)
      (else
        (`KismetArrayLibrary.Array_Add` (`self.AllySpawnerList`) _array_element))))
  (return))

(fn `SpawnCharacterInFormation`
  (params (Formations :type "Array of /Game/Prototype1/Core/Enum/E_Formation Enum (by ref)") (SpawnerType :type "Array of /Game/Prototype1/Core/Characters/BP_CharacterSpawner Object Reference"))
  (bind _output_get (set `self.E_Formation` (`KismetArrayLibrary.Array_Random` Formations)))
  (for _array_element SpawnerType
    (if (`KismetArrayLibrary.Array_Contains` (`/Game/Prototype1/Core/Characters/BP_CharacterSpawner.E_Formation` _array_element) _output_get)
      (if (`/Game/Prototype1/Core/Characters/BP_CharacterSpawner.IsEnemy` _array_element)
        (`KismetArrayLibrary.Array_AddUnique` (`self.EnemyPosition`) _array_element)
        (`/Game/Prototype1/Core/Characters/BP_CharacterSpawner.SpawnUnit` _array_element (`|GetArrayItem` (`self.EnemyCharacterList`) (`KismetMathLibrary.RandomInteger` 2)))
        (else
          (bind _returnvalue (`KismetArrayLibrary.Array_AddUnique` (`self.PartyUnitPosition`) _array_element))
          (`/Game/Prototype1/Core/Characters/BP_CharacterSpawner.SpawnUnit` _array_element (`|GetArrayItem` (`self.PartyUnitCharacterList`) _returnvalue))))
      (else
        (`self.K2_DestroyActor` _array_element))))
  (return))

(fn `UserConstructionScript`
  (`parent.UserConstructionScript`))