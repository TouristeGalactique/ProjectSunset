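; Master GameMode that holds the lists of unlocked heroes and their attributes, with functions to read and update them.
; On BeginPlay it caps the frame rate, then loads attributes from the GameInstance, or adds entries per unlocked hero if none exist, and debug-prints them.
; Save and load events pass both lists through GameInstance messages.
; Adding an unlocked hero saves that list immediately, while adding attributes does not.
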(event `self.ReceiveBeginPlay`
  (`self.SetFPSLimit` 60.0)
  (bind _unitattributes (message `/Game/Prototype1/Core/System/BPI_System.LoadAttributes` (`GameplayStatics.GetGameInstance`)))
  (if (`KismetArrayLibrary.Array_IsEmpty` _unitattributes)
    (for _array_element (`self.HeroesUnlocked`)
      (`self.AddHeroesAttributes` (struct) _array_element))
    (else
      (`self.LoadHeroesAttributes`)))
  (for (_array_element_2 _array_index) (`self.HeroesAttributes`)
    (`KismetSystemLibrary.PrintString` (`KismetStringLibrary.Concat_StrStr` (`|GetEnumeratorNameAsString` (`.UnitName_61_2F3DB50C45E406B373F7C8951DB17F87` (break `/Game/Prototype1/Core/Structures/S_Character_Stats` _array_element_2))) " Ind " (`KismetStringLibrary.Conv_IntToString` _array_index)) true true (struct :`R` 1.0 :`G` 0.042968 :`A` 1.0) 10.0)))

(event `LoadHeroesUnlocked`
  (bind _herounlockednamelist (message `/Game/Prototype1/Core/System/BPI_System.LoadHeroUnlockedList` (`GameplayStatics.GetGameInstance`)))
  (set `self.HeroesUnlocked` _herounlockednamelist))

(event `LoadHeroesAttributes`
  (bind _unitattributes (message `/Game/Prototype1/Core/System/BPI_System.LoadAttributes` (`GameplayStatics.GetGameInstance`)))
  (set `self.HeroesAttributes` _unitattributes))

(event `SaveHeroesUnlocked`
  (message `/Game/Prototype1/Core/System/BPI_System.SaveHeroUnlockedList` (`GameplayStatics.GetGameInstance`) (`self.HeroesUnlocked`)))

(event `SaveHeroesAttributes`
  (message `/Game/Prototype1/Core/System/BPI_System.SaveAttributes` (`GameplayStatics.GetGameInstance`) (`self.HeroesAttributes`)))

(fn `AddHeroesAttributes`
  (params (HeroesAttributes :type "/Game/Prototype1/Core/Structures/S_Character_Stats Structure") (UnitName :type "/Game/Prototype1/Core/Enum/System_Enum/E_CharacterList Enum" :default "NewEnumerator4"))
  (returns (UnusedResult :type Boolean))
  (`KismetArrayLibrary.Array_Add` (`self.HeroesAttributes`) HeroesAttributes)
  (return false))

(fn `AddHeroesUnlocked`
  (params (HeroUnlocked :type "/Game/Prototype1/Core/Enum/System_Enum/E_CharacterList Enum" :default "NewEnumerator4"))
  (returns (UnusedResult :type Boolean))
  (bind _heroesunlocked (`self.HeroesUnlocked`))
  (`KismetArrayLibrary.Array_Insert` _heroesunlocked HeroUnlocked (`KismetArrayLibrary.Array_Length` _heroesunlocked))
  (`self.SaveHeroesUnlocked`)
  (return false))

(fn `GetHeroesAttributes`
  (returns (HeroesUnlocked :type "Array of /Game/Prototype1/Core/Structures/S_Character_Stats Structure"))
  (return (`self.HeroesAttributes`)))

(fn `GetHeroesUnlocked`
  (returns (HeroesUnlocked :type "Array of /Game/Prototype1/Core/Enum/System_Enum/E_CharacterList Enum"))
  (return (`self.HeroesUnlocked`)))

(fn `SetFPSLimit`
  (params (RateLimit :type "Float (single-precision)"))
  (bind _output_get (set `self.FPSLimit` RateLimit))
  (bind _returnvalue (`GameUserSettings.GetGameUserSettings`))
  (`GameUserSettings.SetFrameRateLimit` _returnvalue _output_get)
  (`GameUserSettings.ApplyNonResolutionSettings` _returnvalue)
  (return))

(fn `SetHeroesUnlocked`
  (params (HeroesUnlocked :type "Array of /Game/Prototype1/Core/Enum/System_Enum/E_CharacterList Enum (by ref)" :default _))
  (returns (UnusedResult :type Boolean))
  (set `self.HeroesUnlocked` HeroesUnlocked)
  (return false))

(fn `UserConstructionScript`)