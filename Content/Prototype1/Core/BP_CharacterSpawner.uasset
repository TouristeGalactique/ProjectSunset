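; Spawner actor that creates an AI-controlled BP_Enemy in the level.
; SpawnOneEnemy calls SpawnAIFromClass at the world location and rotation of the I5 box component.
; BeginPlay and the construction script are empty, so spawning relies on that function being called.
; Random placement inside the box and an EnemyPerBattle check exist only as unconnected nodes.
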(event `self.ReceiveBeginPlay`)

(fn `SpawnOneEnemy`
  (bind _i5 (`self.I5`))
  (`AIBlueprintHelperLibrary.SpawnAIFromClass` "/Game/Prototype1/Core/BP_Enemy.BP_Enemy_C" null (`SceneComponent.K2_GetComponentLocation` _i5) (`SceneComponent.K2_GetComponentRotation` _i5) false null)
  (return))

(fn `UserConstructionScript`)